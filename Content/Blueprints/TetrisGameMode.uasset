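; Game mode for a Tetris game that spawns, moves and rotates the falling piece and clears lines.
; Moves are checked against PiecesArray, a flattened width-by-height occupancy grid seeded with floor and wall cells; rotation is unchecked.
; SetPiecesPosition marks a piece's four cells as occupied.
; Before each spawn, VerifyLine line-traces rows from the Destroier actor, hides 11-hit rows, lowers all Piece meshes and shifts the grid down.
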(event `MovePiece`
  (params (x :type "Float (double-precision)") (y :type "Float (double-precision)") (z :type "Float (double-precision)"))
  (bind _currentpiece (`self.CurrentPiece`))
  (bind _canmove (`self.canMovePiece` (`/Game/Blueprints/piece.Meshes` _currentpiece) x z))
  (if (and (not _canmove) (< z 0.0))
    (`/Game/Blueprints/piece.StopPiece` _currentpiece)
    (`KismetSystemLibrary.PrintString` (`KismetStringLibrary.Concat_StrStr` (`KismetStringLibrary.Conv_BoolToString` _canmove) " moverr"))
    (elif (and (`/Game/Blueprints/piece.isMoving` _currentpiece) _canmove)
      (`self.K2_AddActorWorldTransform` _currentpiece (`KismetMathLibrary.MakeTransform` (`KismetMathLibrary.MakeVector` x 0.0 z)) false false))))

(event `self.ReceiveBeginPlay`
  (`self.CreatePiece`)
  (for _ (range (* (`self.heightInBlocks`) (`self.widthInBlocks`)))
    (`KismetArrayLibrary.Array_Add` (`self.PiecesArray`)))
  (`self.setFloorWallsPiecesArray`))

(event `RotatePiece`
  (`self.K2_AddActorWorldRotation` (`self.CurrentPiece`) (`KismetMathLibrary.MakeRotator` 0.0 90.0) false false))

(event `CreatePiece`
  (if (and (> (- (`GameplayStatics.GetTimeSeconds`) (`self.timePieceCreated`)) 0.2) (not (`self.blockCreate`)))
    (`self.VerifyLine`)
    (bind _returnvalue (`|SpawnActorFromClass` "/Game/Blueprints/piece.piece_C" (`KismetMathLibrary.MakeTransform` (500.0 0.0 2000.0)) "Undefined" "OverrideRootScale" null null))
    (set `self.CurrentPiece` _returnvalue)
    (set `self.timePieceCreated` (`GameplayStatics.GetTimeSeconds`))
    (else
      (`KismetSystemLibrary.PrintString` "Hello"))))

(event `setWallsPositions`
  (bind _heightinblocks (`self.heightInBlocks`))
  (bind _returnvalue (/ (* _heightinblocks 10.0) 2.0))
  (`SceneComponent.K2_SetWorldTransform` (`StaticMeshActor.StaticMeshComponent` (`self.Wall1`)) (`KismetMathLibrary.MakeTransform` (`KismetMathLibrary.MakeVector` 50.0 0.0 _returnvalue) (struct) (`KismetMathLibrary.MakeVector` 0.25 5.0 (`KismetMathLibrary.Conv_IntToDouble` _heightinblocks))) false false)
  (`SceneComponent.K2_SetWorldTransform` (`StaticMeshActor.StaticMeshComponent` (`self.Wall2`)) (`KismetMathLibrary.MakeTransform` (`KismetMathLibrary.MakeVector` (- (* (`self.widthInBlocks`) 10.0) 50.0) 0.0 _returnvalue) (struct) (`KismetMathLibrary.MakeVector` 0.25 5.0 (`KismetMathLibrary.Conv_IntToDouble` _heightinblocks))) false false))

(event `self.ReceiveTick`
  (params (DeltaSeconds :type "Float (single-precision)")))

(event `VerifyLine`
  (bind (_returnvalue_x _returnvalue_y _returnvalue_z) (`KismetMathLibrary.BreakVector` (`self.K2_GetActorLocation` (`self.Destroier`))))
  (bind (_returnvalue_x_2 _returnvalue_y_2 _returnvalue_z_2) (`KismetMathLibrary.BreakVector` (`self.K2_GetActorLocation` (`self.Destroier`))))
  (for _index (range 1 20)
    (bind _returnvalue (* (`KismetMathLibrary.Conv_IntToDouble` _index) _returnvalue_z))
    (bind _outhits (`KismetSystemLibrary.LineTraceMulti` :`Start` (`KismetMathLibrary.MakeVector` _returnvalue_x _returnvalue_y _returnvalue) :`End` (`KismetMathLibrary.MakeVector` 1822.0 0.0 _returnvalue) :`TraceChannel` "TraceTypeQuery1" :`DrawDebugType` "ForDuration" :`TraceHitColor` (struct :`R` 0.213542 :`A` 1.0) :`DrawTime` 1.0))
    (if (== (`KismetArrayLibrary.Array_Length` _outhits) 11)
      (for _array_element _outhits
        (bind (_bblockinghit _binitialoverlap _time _distance _location _impactpoint _normal _impactnormal _physmat _hitactor _hitcomponent) (`GameplayStatics.BreakHitResult` _array_element))
        (`SceneComponent.SetHiddenInGame` _hitcomponent true false)
        (`PrimitiveComponent.SetCollisionEnabled` _hitcomponent "NoCollision")
        (`KismetSystemLibrary.Delay` 0.2)
        (bind _outactors (`GameplayStatics.GetAllActorsOfClass` "/Game/Blueprints/piece.piece_C"))
        (set `self.blockCreate` true)
        ;[1 1 1] Move as pecas para baixo
        (for _array_element_2 _outactors
          (for _array_element_3 (`/Game/Blueprints/piece.Meshes` _array_element_2)
            (`SceneComponent.K2_AddWorldTransform` _array_element_3 (`KismetMathLibrary.MakeTransform` (0.0 0.0 -100.0)) false false)))
        (set `self.blockCreate` false)
        (`self.actualizePiecesPosition` (`KismetMathLibrary.FTrunc` (/ _returnvalue_z_2 100.0)))))))

(fn `actualizePiecesPosition`
  (params (TargetLine :type Integer))
  (bind _piecesarray (`self.PiecesArray`))
  (bind _widthinblocks (`self.widthInBlocks`))
  ;[1 1 1] esta funcao sera chamada quando houver uma linha de meshes destuida
  (for _index (range (* TargetLine _widthinblocks) (+ (* _widthinblocks (`self.heightInBlocks`)) 1))
    ;[1 1 1] Verifica no array onde há posicoes ocupadas ('1') e tire-as colocando '0'
    (if (== (`|GetArrayItem` _piecesarray _index) 1)
      (`KismetArrayLibrary.Array_Set` _piecesarray _index)
      ;[1 1 1] Coloque como posicao ocupada (1), a posicao logo abaixo daquela que foi destruida
      (`KismetArrayLibrary.Array_Set` _piecesarray (- _index (`self.widthInBlocks`)) 1)))
  (`self.setFloorWallsPiecesArray`))

(fn `canMovePiece`
  (params (Meshes :type "Array of StaticMeshComponent Object Reference") (displacement_X :type "Float (double-precision)") (displacement_Z :type "Float (double-precision)") (NewParam :type Integer))
  (returns (canMove :type Boolean))
  (bind _returnvalue (/ displacement_X 100.0))
  (bind _returnvalue_2 (/ displacement_Z 100.0))
  (bind _widthinblocks (`self.widthInBlocks`))
  (bind (_returnvalue_x _returnvalue_y _returnvalue_z) (`KismetMathLibrary.BreakVector` (`SceneComponent.K2_GetComponentLocation` (`|GetArrayItem` Meshes 3))))
  (bind (_returnvalue_x_2 _returnvalue_y_2 _returnvalue_z_2) (`KismetMathLibrary.BreakVector` (`SceneComponent.K2_GetComponentLocation` (`|GetArrayItem` Meshes))))
  (bind (_returnvalue_x_3 _returnvalue_y_3 _returnvalue_z_3) (`KismetMathLibrary.BreakVector` (`SceneComponent.K2_GetComponentLocation` (`|GetArrayItem` Meshes 1))))
  (bind (_returnvalue_x_4 _returnvalue_y_4 _returnvalue_z_4) (`KismetMathLibrary.BreakVector` (`SceneComponent.K2_GetComponentLocation` (`|GetArrayItem` Meshes 2))))
  ;[1 1 1] se a posicao no array PiecesArray da mesh tiver '1' significa que nesta posicao já encontra-se uma mesh parada e portanto a peca nao pode se mover no sentido deste deslocamento.
  (for _index (range 4)
    (if (== (`|GetArrayItem` (`self.PiecesArray`) (`|GetArrayItem` (`|MakeArray` (`KismetMathLibrary.FTrunc` (+ (* _widthinblocks (+ (/ _returnvalue_z_2 100.0) _returnvalue_2)) (+ (/ _returnvalue_x_2 100.0) _returnvalue))) (`KismetMathLibrary.FTrunc` (+ (* _widthinblocks (+ (/ _returnvalue_z_3 100.0) _returnvalue_2)) (+ (/ _returnvalue_x_3 100.0) _returnvalue))) (`KismetMathLibrary.FTrunc` (+ (* _widthinblocks (+ (/ _returnvalue_z_4 100.0) _returnvalue_2)) (+ (/ _returnvalue_x_4 100.0) _returnvalue))) (`KismetMathLibrary.FTrunc` (+ (* _widthinblocks (+ (/ _returnvalue_z 100.0) _returnvalue_2)) (+ (/ _returnvalue_x 100.0) _returnvalue)))) _index)) 1)
      (return false)))
  (return true))

(fn `setPiecesPosition`
  (params (Meshes :type "Array of StaticMeshComponent Object Reference"))
  (bind _aux (`self.aux`))
  (bind _piecesarray (`self.PiecesArray`))
  (for _index (range 4)
    (`KismetArrayLibrary.Array_Set` _piecesarray (`|GetArrayItem` (`|MakeArray` (`self.GetPiecesPositions` 0 Meshes) (`self.GetPiecesPositions` 1 Meshes) (`self.GetPiecesPositions` 2 Meshes) (`self.GetPiecesPositions` 3 Meshes)) _index) 1))
  ;[1 1 1] Debug piecesarray
  (set `self.aux` 0)
  (for _ (range 11)
    (`KismetSystemLibrary.PrintString` (`KismetStringLibrary.Concat_StrStr` (`KismetStringLibrary.Conv_IntToString` (`|GetArrayItem` _piecesarray _aux)) (`KismetStringLibrary.Conv_IntToString` (`|GetArrayItem` _piecesarray (+ _aux 1))) (`KismetStringLibrary.Conv_IntToString` (`|GetArrayItem` _piecesarray (+ _aux 2))) (`KismetStringLibrary.Conv_IntToString` (`|GetArrayItem` _piecesarray (+ _aux 3))) (`KismetStringLibrary.Conv_IntToString` (`|GetArrayItem` _piecesarray (+ _aux 4))) (`KismetStringLibrary.Conv_IntToString` (`|GetArrayItem` _piecesarray (+ _aux 5))) (`KismetStringLibrary.Conv_IntToString` (`|GetArrayItem` _piecesarray (+ _aux 6))) (`KismetStringLibrary.Conv_IntToString` (`|GetArrayItem` _piecesarray (+ _aux 7))) (`KismetStringLibrary.Conv_IntToString` (`|GetArrayItem` _piecesarray (+ _aux 8))) (`KismetStringLibrary.Conv_IntToString` (`|GetArrayItem` _piecesarray (+ _aux 9))) (`KismetStringLibrary.Conv_IntToString` (`|GetArrayItem` _piecesarray (+ _aux 10))) (`KismetStringLibrary.Conv_IntToString` (`|GetArrayItem` _piecesarray (+ _aux 11)))) true true (struct :`G` 0.66 :`B` 1.0 :`A` 1.0) 10.0)
    (set `self.aux` (+ (`self.aux`) (`self.widthInBlocks`))))
  (`KismetSystemLibrary.PrintText` "Top^"))

(fn `UserConstructionScript`)