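; Tetris piece actor made of four meshes that falls in timed steps until it lands.
; The construction script picks one of seven shapes at random, setting mesh offsets and a matching color.
; Tick asks TetrisGameMode to move the piece down every half second.
; Overlapping FloorCube (matched by display name) or StopPiece halts it, registers its meshes and requests a new piece, height-gated for the overlap case.
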(event `self.ReceiveBeginPlay`
  ;[1 1 1] Aloca as 4 meshes em um array de meshes
  (bind _result (`BlueprintSetLibrary.Set_ToArray` (`|MakeSet` (`self.Mesh1`) (`self.Mesh2`) (`self.Mesh3`) (`self.Mesh4`))))
  (set `self.Meshes` _result)
  ;[1 1 1] Guarda o Game Mode em uma variavel, pois ele sera muito utilizado
  (bind _astetris_game_mode (cast `/Game/Blueprints/TetrisGameMode` (`GameplayStatics.GetGameMode`)))
  (set `self.TetrisGameMode` _astetris_game_mode)
  ;[1 1 1] Ignora a colisao das meshs com o proprio actor da qual elas pertencem
  (`PrimitiveComponent.IgnoreActorWhenMoving` (`self.Mesh1`) self true)
  (`PrimitiveComponent.IgnoreActorWhenMoving` (`self.Mesh2`) self true)
  (`PrimitiveComponent.IgnoreActorWhenMoving` (`self.Mesh3`) self true)
  (`PrimitiveComponent.IgnoreActorWhenMoving` (`self.Mesh4`) self true))

(event `self.ReceiveActorBeginOverlap`
  (params (OtherActor :type "Actor Object Reference"))
  (bind (_returnvalue_x _returnvalue_y _returnvalue_z) (`KismetMathLibrary.BreakVector` (`SceneComponent.K2_GetComponentLocation` (`self.DefaultSceneRoot`))))
  (if (`KismetStringLibrary.EqualEqual_StrStr` (`KismetSystemLibrary.GetDisplayName` OtherActor) "FloorCube")
    (set `self.isMoving` false)
    (`/Game/Blueprints/TetrisGameMode.setPiecesPosition` (`self.TetrisGameMode`) (`self.Meshes`))
    (if (<= _returnvalue_z 2000.0)
      (`/Game/Blueprints/TetrisGameMode.CreatePiece` (`self.TetrisGameMode`)))))

(event `self.ReceiveTick`
  (params (DeltaSeconds :type "Float (single-precision)"))
  (bind _returnvalue (`GameplayStatics.GetTimeSeconds`))
  (if (and (`self.isMoving`) (>= (- _returnvalue (`self.Time`)) 0.5))
    (set `self.Time` _returnvalue)
    (`/Game/Blueprints/TetrisGameMode.MovePiece` (`self.TetrisGameMode`) 0.0 0.0 -100.0)))

(event `StopPiece`
  (bind _tetrisgamemode (`self.TetrisGameMode`))
  (set `self.isMoving` false)
  (`/Game/Blueprints/TetrisGameMode.setPiecesPosition` _tetrisgamemode (`self.Meshes`))
  (`/Game/Blueprints/TetrisGameMode.CreatePiece` _tetrisgamemode))

(fn `setMaterial`
  (params (Material :type "MaterialInterface Object Reference"))
  (`PrimitiveComponent.SetMaterial` (`self.Mesh2`) 0 Material)
  (`PrimitiveComponent.SetMaterial` (`self.Mesh3`) 0 Material)
  (`PrimitiveComponent.SetMaterial` (`self.Mesh4`) 0 Material)
  (`PrimitiveComponent.SetMaterial` (`self.Mesh1`) 0 Material))

(fn `setPiece`
  (params (parameters :type "Array of Float (double-precision)"))
  (`SceneComponent.K2_SetRelativeLocation` (`self.Mesh1`) (`KismetMathLibrary.MakeVector` (`|GetArrayItem` parameters) (`|GetArrayItem` parameters 1) (`|GetArrayItem` parameters 2)) false false)
  (`SceneComponent.K2_SetRelativeLocation` (`self.Mesh2`) (`KismetMathLibrary.MakeVector` (`|GetArrayItem` parameters 3) (`|GetArrayItem` parameters 4) (`|GetArrayItem` parameters 5)) false false)
  (`SceneComponent.K2_SetRelativeLocation` (`self.Mesh3`) (`KismetMathLibrary.MakeVector` (`|GetArrayItem` parameters 6) (`|GetArrayItem` parameters 7) (`|GetArrayItem` parameters 8)) false false)
  (`SceneComponent.K2_SetRelativeLocation` (`self.Mesh4`) (`KismetMathLibrary.MakeVector` (`|GetArrayItem` parameters 9) (`|GetArrayItem` parameters 10) (`|GetArrayItem` parameters 11)) false false))

(fn `UserConstructionScript`
  (switch `int` (`KismetMathLibrary.RandomIntegerInRange` 0 6)
    (:`0`
      (`self.setPiece` (`self.Piece1`))
      (`self.setMaterial` "/Game/Materials/MaterialBlue.MaterialBlue"))
    (:`1`
      (`self.setPiece` (`self.Piece2`))
      (`self.setMaterial` "/Game/Materials/MaterialDarkBlue.MaterialDarkBlue"))
    (:`2`
      (`self.setPiece` (`self.Piece3`))
      (`self.setMaterial` "/Game/Materials/MaterialDarkGreen.MaterialDarkGreen"))
    (:`3`
      (`self.setPiece` (`self.Piece4`))
      (`self.setMaterial` "/Game/Materials/MaterialGreen.MaterialGreen"))
    (:`4`
      (`self.setPiece` (`self.Piece5`))
      (`self.setMaterial` "/Game/Materials/MaterialoRANGE.MaterialOrange"))
    (:`5`
      (`self.setPiece` (`self.Piece6`))
      (`self.setMaterial` "/Game/Materials/MaterialRed.MaterialRed"))
    (:`6`
      (`self.setPiece` (`self.Piece7`))
      (`self.setMaterial` "/Game/Materials/MaterialYellow.MaterialYellow"))))